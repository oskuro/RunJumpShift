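; Elevator actor Blueprint with two sliding doors that open when anything begins overlapping its trigger collision.
; OpenDoors plays a timeline that lerps both doors apart along their relative Y axis between fixed positions.
; CloseDoors records each door's current Y and lerps it back to closed on a second timeline, but nothing in this file triggers it.
; The file contains no logic for moving the elevator itself.
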(event OnComponentBeginOverlap(OpenDoorsCollision)
  (params (OverlappedComponent :type Primitive%20Component%20Object%20Reference) (OtherActor :type Actor%20Object%20Reference) (OtherComp :type Primitive%20Component%20Object%20Reference) (OtherBodyIndex :type Integer) (bFromSweep :type Boolean) (SweepResult :type Hit%20Result%20Structure%20%28by%20ref%29))
  (CallFunction|OpenDoors))

(event Custom|OpenDoors
  (bind _doorright (Variables|Default|GetDoorRight))
  (bind _doorleft (Variables|Default|GetDoorLeft))
  (bind _relativelocation (Variables|/Script/Engine.SceneComponent|GetRelativeLocation _doorright))
  (bind _relativelocation_2 (Variables|/Script/Engine.SceneComponent|GetRelativeLocation _doorleft))
  (bind _lerp (Timeline|Timeline_0 PlayFromStart)
    (:Update
      (Transformation|SetRelativeLocation _doorright (Math|Vector|MakeVector (.x _relativelocation) (Math|Float|Lerp 0.0 -1.7e+02 _lerp) (.z _relativelocation)) false false)
      (Transformation|SetRelativeLocation _doorleft (Math|Vector|MakeVector (.x _relativelocation_2) (Math|Float|Lerp 2e+02 3.7e+02 _lerp) (.z _relativelocation_2)) false false))))

(event Custom|CloseDoors
  (bind _doorleft (Variables|Default|GetDoorLeft))
  (bind _doorright (Variables|Default|GetDoorRight))
  (bind _relativelocation (Variables|/Script/Engine.SceneComponent|GetRelativeLocation _doorright))
  (bind _relativelocation_2 (Variables|/Script/Engine.SceneComponent|GetRelativeLocation _doorleft))
  (Variables|Default|SetyStartRightDoor (.y (Variables|/Script/Engine.SceneComponent|GetRelativeLocation (Variables|Default|GetDoorRight))))
  (Variables|Default|SetyStartLeftDoor (.y (Variables|/Script/Engine.SceneComponent|GetRelativeLocation (Variables|Default|GetDoorLeft))))
  (bind _lerp (Timeline|Timeline_1 PlayFromStart)
    (:Update
      (Transformation|SetRelativeLocation _doorright (Math|Vector|MakeVector (.x _relativelocation) (Math|Float|Lerp (Variables|Default|GetyStartRightDoor) 0.0 _lerp) (.z _relativelocation)) false false)
      (Transformation|SetRelativeLocation _doorleft (Math|Vector|MakeVector (.x _relativelocation_2) (Math|Float|Lerp (Variables|Default|GetyStartLeftDoor) 2e+02 _lerp) (.z _relativelocation_2)) false false))))

(fn ConstructionScript)